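; Enemy AI character that runs the Enemy_BT behavior tree and shoots at the first-person player.
; BeginPlay starts a delay-driven loop that line traces forward along control rotation and, on hitting FirstPersonCharacter, calls Fire, gated by a ShotReadyAI cooldown.
; Fire plays a montage and sound and spawns EnemyAIProjectile, aimed by the FirstPersonCamera rotation.
; HealthDepleetAI subtracts fixed damage, prints health and destroys the actor at zero.
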(event EventBeginPlay
  (bind _returnvalue (Transformation|GetActorLocation))
  (bind (_x _y _z) (Math|Vector|BreakVector _returnvalue))
  (bind _returnvalue_2 (+ _z 3e+01))
  (bind _returnvalue_3 (Math|Vector|MakeVector _x _y _returnvalue_2))
  (AI|RunBehaviorTree (AI|GetAIController self) "/Game/Ai/Enemy_BT.Enemy_BT")
  (Utilities|FlowControl|Delay 1.0 :!label _label)
  (bind _outhit (Collision|LineTraceByChannel _returnvalue_3 (+ _returnvalue_3 (* (Math|Rotator|GetRotationXVector (Pawn|GetControlRotation :!class /Script/Engine.Pawn)) 2.5e+03)) "TraceTypeQuery1" false 0 "ForDuration" true "(R=1.000000,G=0.000000,B=0.000000,A=1.000000)" "(R=1.000000,G=0.987220,B=0.522989,A=1.000000)"))
  (Utilities|Casting|CastToFirstPersonCharacter (.HitActor (Collision|BreakHitResult _outhit))
    (:then
      (if (Variables|Default|GetShotReadyAI)
        (Variables|Default|SetShotReadyAI false)
        (CallFunction|Fire)
        (Utilities|FlowControl|Delay 2.0)
        (Variables|Default|SetShotReadyAI true)
        (goto _label)))
    (:CastFailed
      (goto _label))))

(fn ConstructionScript
  (|CallParentFunction))

(fn Fire
  (bind _firstpersoncamera (Variables|Default|GetFirstPersonCamera))
  (bind _returnvalue (Transformation|GetWorldRotation _firstpersoncamera))
  (Animation|Montage|MontagePlay (Components|SkeletalMesh|GetAnimInstance (Variables|Default|GetMesh2P)) "/Game/FirstPerson/Animations/FirstPersonFire_Montage.FirstPersonFire_Montage" 1.0 "MontageLength" 0.0 true)
  (Game|SpawnActorfromClass "/Game/Ai/EnemyAIProjectile.EnemyAIProjectile_C" (Math|Transform|MakeTransform (+ (Transformation|GetWorldLocation (Variables|Default|GetSphere)) (Math|Vector|RotateVector (Variables|Default|GetGunOffset) _returnvalue)) _returnvalue) "AdjustIfPossibleButDontSpawnIfColliding" 0 0) ; Spawn projectile
  (Audio|PlaySoundatLocation "/Game/FirstPerson/Audio/FirstPersonTemplateWeaponFire02.FirstPersonTemplateWeaponFire02" (Transformation|GetActorLocation) "0, 0, 0" 1.0 1.0 0.0 0 0 0) ; Play firing sound
)

(fn HealthDepleetAI
  (if (> (Variables|Default|GetHealthAi) 0.0)
    (Variables|Default|SetHealthAi (- (Variables|Default|GetHealthAi) 5.0))
    (Development|PrintString (Utilities|String|ToString(Float) (Variables|Default|GetHealthAi)))
    (if (not (> (Variables|Default|GetHealthAi) 0.0))
      (Actor|DestroyActor))
    (else
      (Actor|DestroyActor))))