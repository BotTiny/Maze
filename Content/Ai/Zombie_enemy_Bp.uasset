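; Zombie enemy character that chases the first-person player while they overlap it and plays an attack montage in reach.
; AI MoveTo re-triggers itself after attacks or failed moves, with a delay gating attack rate.
; Player damage comes from the CheckForProjectile component's overlap, not the montage.
; AnyDamage and fixed-step HealthDepleate both reduce health and destroy it, but only HealthDepleate increments the game mode's mummy score.
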(event OnComponentBeginOverlap(CheckforProjectile)
  (params (OverlappedComponent :type Primitive%20Component%20Object%20Reference) (OtherActor :type Actor%20Object%20Reference) (OtherComp :type Primitive%20Component%20Object%20Reference) (OtherBodyIndex :type Integer) (bFromSweep :type Boolean) (SweepResult :type Hit%20Result%20Structure%20%28by%20ref%29))
  (bind _asfirst_person_character (Utilities|Casting|CastToFirstPersonCharacter OtherActor))
  (Default|HealthDepleatPlayer _asfirst_person_character))

(event Custom|Chase%20The%20Player
  ;[1 1 1] Chase player
  (AI|AIMoveTo self "0, 0, 0" (Game|GetPlayerCharacter 0) 1e+02 false
    (:OnSuccess
      (if (Variables|Default|GetCan%20Attack)
        (Variables|Default|SetCan%20Attack false)
        (Animation|Montage|PlayMontage (Variables|Character|GetMesh) 0
          (:then
            (Utilities|FlowControl|Delay (Variables|Default|GetAttack%20Rate))
            (Variables|Default|SetCan%20Attack true))
          (:OnCompleted
            (if (Variables|Default|GetPlayer%20In%20Rnage)
              (CallFunction|ChasethePlayer))))
        (else
          (CallFunction|ChasethePlayer))))
    (:OnFail
      (Utilities|FlowControl|Delay 2.0)
      (if (Variables|Default|GetPlayer%20In%20Rnage)
        (CallFunction|ChasethePlayer)))))

(event Game|Damage|EventAnyDamage
  (params (Damage :type Float%20%28single-precision%29) (DamageType :type Damage%20Type%20Object%20Reference) (InstigatedBy :type Controller%20Object%20Reference) (DamageCauser :type Actor%20Object%20Reference))
  ;[1 1 1] Take Dmg, and destroy
  (bind _output_get (Variables|Default|SetHealth (- (Variables|Default|GetHealth) Damage)))
  (if (<= _output_get 0.0)
    (Actor|DestroyActor)
    (else
      (Development|PrintString (Utilities|String|ToString(Float) (Variables|Default|GetHealth))))))

(event Collision|EventActorBeginOverlap
  (params (OtherActor :type Actor%20Object%20Reference))
  ;[1 1 1] Start Chasing player
  (Utilities|Casting|CastToFirstPersonCharacter OtherActor)
  (Variables|Default|SetPlayer%20In%20Rnage true)
  (CallFunction|ChasethePlayer))

(event Collision|EventActorEndOverlap
  (params (OtherActor :type Actor%20Object%20Reference))
  ;[1 1 1] Stop Chasing Player
  (Utilities|Casting|CastToFirstPersonCharacter OtherActor)
  (Variables|Default|SetPlayer%20In%20Rnage false)
  (Components|Movement|StopMovementImmediately (Variables|Character|GetCharacterMovement))
  (Development|PrintString "No player"))

(fn ConstructionScript)

(fn HealthDepleate
  (if (> (Variables|Default|GetHealth) 0.0)
    (Variables|Default|SetHealth (- (Variables|Default|GetHealth) 2e+01))
    (Development|PrintString (Utilities|String|ToString(Float) (Variables|Default|GetHealth)))
    (if (not (> (Variables|Default|GetHealth) 0.0))
      (bind _asfirst_person_game_mode (Utilities|Casting|CastToFirstPersonGameMode (Game|GetGameMode)))
      (Default|IncraseScoreMummy _asfirst_person_game_mode)
      (Actor|DestroyActor))
    (else
      (bind _asfirst_person_game_mode_2 (Utilities|Casting|CastToFirstPersonGameMode (Game|GetGameMode)))
      (Default|IncraseScoreMummy _asfirst_person_game_mode_2)
      (Actor|DestroyActor))))