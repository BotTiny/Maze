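; BP_EnemyController is an AI controller for enemies that starts the Enemy_BT behavior tree on BeginPlay.
; Its AI Perception component writes each stimulus update into the Blackboard for the tree to use.
; Sight updates store the perceived actor as TargetActor, while any other sense stores the stimulus location as TargetLocation.
; It does not check whether the stimulus was successfully sensed, so sight loss also sets TargetActor.
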(event OnTargetPerceptionUpdated(AIPerception)
  (params (Actor :type Actor%20Object%20Reference) (Stimulus :type AI%20Stimulus%20Structure))
  (bind _returnvalue (Class|AIPerceptionSystem|GetSenseClassforStimulus Stimulus))
  (if (== _returnvalue "/Script/AIModule.AISense_Sight")
    (AI|Components|Blackboard|SetValueasObject (Variables|Default|GetBlackboard) (Utilities|Name|MakeLiteralName "TargetActor") Actor)
    (else
      (AI|Components|Blackboard|SetValueasVector (Variables|Default|GetBlackboard) (Utilities|Name|MakeLiteralName "TargetLocation") (.StimulusLocation (Utilities|Struct|BreakAIStimulus Stimulus))))))

(event EventBeginPlay
  (|CallParentFunction)
  (AI|RunBehaviorTree "/Game/Ai/Enemy_BT.Enemy_BT"))

(fn ConstructionScript
  (|CallParentFunction))